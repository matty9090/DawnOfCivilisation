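; Planet actor that applies materials to its terrain and water Geosphere child actors and populates the terrain with forests of trees.
; On BeginPlay, random terrain vertices become forest centers for PlaceForest.
; PlaceForest projects 2D GeneratePoints samples onto each vertex's tangent plane, traces along the inverted normal, and spawns surface-aligned trees only on terrain hits.
; Releasing left mouse traces from the camera and spawns a full-scale tree on the hit surface.
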(event `self.ReceiveBeginPlay`
  (bind _asgeosphere (cast `Geosphere` (`ChildActorComponent.ChildActor` (`self.Terrain`))))
  (set `self.TerrainSphere` _asgeosphere)
  (`self.EnableInput` (`GameplayStatics.GetPlayerController` 0))
  (bind _vertices (`Geosphere.GetVertices` _asgeosphere))
  (for _ (range (+ (`self.NumForests`) 1))
    (bind _output_get (set `self.RandomNumber` (`KismetMathLibrary.RandomInteger` (`KismetArrayLibrary.Array_Length` _vertices))))
    (bind _returnvalue (`Geosphere.GetNormal` (`self.TerrainSphere`) _output_get))
    (`self.PlaceForest` (`|GetArrayItem` _vertices _output_get) _returnvalue (`self.ForestRadius`))))

(event `Key|LeftMouseButton`
  (params (Key :type "Key Structure"))
  (bind _returnvalue (`GameplayStatics.GetPlayerCameraManager` 0))
  (bind _returnvalue_2 (`PlayerCameraManager.GetCameraLocation` _returnvalue))
  (:`Released`
    (bind (_outhit _returnvalue_3) (`KismetSystemLibrary.LineTraceSingleForObjects` :`Start` _returnvalue_2 :`End` (+ _returnvalue_2 (* (`self.GetActorForwardVector` _returnvalue) 6000.0)) :`ObjectTypes` (`|MakeArray` "ObjectTypeQuery1" "ObjectTypeQuery2" :!type "EObjectTypeQuery Enum") :`bIgnoreSelf` false))
    (if _returnvalue_3
      (bind (_bblockinghit _binitialoverlap _time _distance _location _impactpoint _normal) (`GameplayStatics.BreakHitResult` _outhit))
      (`|SpawnActorFromClass` "/Game/Blueprints/Tree.Tree_C" (`KismetMathLibrary.MakeTransform` _location (`KismetMathLibrary.MakeRotFromZ` _normal)) "Undefined" "OverrideRootScale" null null))))

(fn `PlaceForest`
  (params (Position :type "Vector Structure") (Normal :type "Vector Structure") (ForestRadius :type "Float (double-precision)"))
  (locals (Pos :type "Vector Structure") (Points :type "Vector Structure") (StartPoint :type "Vector Structure" :default (0.0 0.0 0.0)) (Axis1 :type "Vector Structure" :default (0.0 0.0 0.0)) (Axis2 :type "Vector Structure" :default (0.0 0.0 0.0)))
  (bind _returnvalue (/ (`self.ForestRadius`) 2.0))
  (bind _returnvalue_2 (`PoissonDiscSampling.GeneratePoints` (`self.TreeRadius`) ForestRadius (`self.Threshold`) (`self.Frequency`) (/ (`self.FadePercent`) 100.0)))
  (set `local.StartPoint` (+ Position (* Normal 300.0)))
  (bind _output_get (set `local.Axis1` (`KismetMathLibrary.Normal` (`KismetMathLibrary.Cross_VectorVector` Normal (0.0 1.0 0.0)))))
  (set `local.Axis2` (`KismetMathLibrary.Normal` (`KismetMathLibrary.Cross_VectorVector` _output_get Normal)))
  (for _array_element _returnvalue_2
    (bind (_x _y) (`KismetMathLibrary.BreakVector2D` _array_element))
    (bind _returnvalue_3 (+ (`local.StartPoint`) (* (`local.Axis1`) (- _x _returnvalue)) (* (`local.Axis2`) (- _y _returnvalue))))
    (bind (_outhit _returnvalue_4) (`KismetSystemLibrary.LineTraceSingle` :`Start` _returnvalue_3 :`End` (+ _returnvalue_3 (* (`local.Normal`) -1000.0)) :`TraceChannel` "TraceTypeQuery1" :`bIgnoreSelf` false :`DrawTime` 60.0))
    (if _returnvalue_4
      (bind (_bblockinghit _binitialoverlap _time _distance _location _impactpoint _normal _impactnormal _physmat _hitactor) (`GameplayStatics.BreakHitResult` _outhit))
      (if (== _hitactor (`ChildActorComponent.ChildActor` (`self.Terrain`)))
        (`|SpawnActorFromClass` "/Game/Blueprints/Tree.Tree_C" (`KismetMathLibrary.MakeTransform` _location (`KismetMathLibrary.MakeRotFromZ` _normal) (0.32 0.32 0.32)) "Undefined" "OverrideRootScale" null null)))))

(fn `UserConstructionScript`
  (bind _asgeosphere (cast `Geosphere` (`ChildActorComponent.ChildActor` (`self.Terrain`))))
  (`PrimitiveComponent.SetMaterial` (`Geosphere.Mesh` _asgeosphere) 0 (`self.TerrainMaterial`))
  (bind _asgeosphere_2 (cast `Geosphere` (`ChildActorComponent.ChildActor` (`self.Water`))))
  (`PrimitiveComponent.SetMaterial` (`Geosphere.Mesh` _asgeosphere_2) 0 (`self.WaterMaterial`)))