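; Alien actor that idles on a planet and can be told to walk to a node on the terrain's node graph.
; WalkTo pathfinds from the closest node to the target, stores the path and starts the walk animation.
; On the next Tick it issues AI move requests for every path node in a single loop without waiting for arrival, then immediately returns to idle state and animation.
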(event `self.ReceiveBeginPlay`
  (bind _terrain (`/Game/Blueprints/Planet.GetTerrainRef` (`self.Planet`)))
  (set `self.NodeGraph` (`Geosphere.NodeGraph` _terrain))
  (`SkeletalMeshComponent.PlayAnimation` (`self.SkeletalMeshComponent`) "/Game/Models/Alien/Alien_Anim_AlienRig_Idle.Alien_Anim_AlienRig_Idle" true))

(event `self.ReceiveTick`
  (params (DeltaSeconds :type "Float (single-precision)"))
  (bind _path (`self.Path`))
  (bind _currentnode (`self.CurrentNode`))
  (if (`|EnumEquality` (`self.State`) "NewEnumerator2")
    (set `self.State` "NewEnumerator0")
    (`AIBlueprintHelperLibrary.SimpleMoveToLocation` (`AIBlueprintHelperLibrary.GetAIController` self) (`GraphNode.Position` (`|GetArrayItem` _path (`self.CurrentNode`))) :!label _label)
    (if (>= _currentnode (- (`KismetArrayLibrary.Array_Length` _path) 1))
      (set `self.State` "NewEnumerator0")
      (`SkeletalMeshComponent.PlayAnimation` (`self.SkeletalMeshComponent`) "/Game/Models/Alien/Alien_Anim_AlienRig_Idle.Alien_Anim_AlienRig_Idle" true)
      (else
        (`/Engine/EditorBlueprintResources/StandardMacros.IncrementInt` _currentnode
          (:`  `
            (goto _label)))))))

(fn `UserConstructionScript`)

(fn `WalkTo`
  (params (Node :type Integer))
  (bind _nodegraph (`self.NodeGraph`))
  (`KismetSystemLibrary.PrintString` (`KismetStringLibrary.Concat_StrStr` "Walking to node " (`KismetStringLibrary.Conv_IntToString` Node)))
  (bind _index (`NodeGraph.GetClosestNode` _nodegraph (`self.K2_GetActorLocation`) 200.0))
  (bind _path (`NodeGraph.Pathfind` _nodegraph _index Node))
  (set `self.Path` _path)
  (set `self.CurrentNode` 0)
  (set `self.State` "NewEnumerator2")
  (`SkeletalMeshComponent.PlayAnimation` (`self.SkeletalMeshComponent`) "/Game/Models/Alien/Alien_Anim_AlienRig_Walking.Alien_Anim_AlienRig_Walking" true))