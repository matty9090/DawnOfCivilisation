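; Alien worker character that walks a planet's node graph and constructs its assigned building.
; A Tick-driven Idle/Building/Walking state machine swaps looping animations, with WalkTo pathfinding from the nearest node on the terrain's graph.
; Walking sweeps along the path oriented radially from the world origin, switching to Building on hitting the assigned building or Idle at path end.
; Building advances construction by frame time and build speed until BuildBuilding returns true.
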(event `self.ReceiveBeginPlay`
  (bind _terrain (`/Game/Blueprints/Planet/PlanetBP.GetTerrainRef` (`self.Planet`)))
  (set `self.NodeGraph` (`Geosphere.NodeGraph` _terrain))
  (`self.StateSetIdle`))

(event `self.ReceiveTick`
  (params (DeltaSeconds :type "Float (single-precision)"))
  (switch `/Game/Blueprints/Alien/AlienState` (`self.State`)
    (:`NewEnumerator0`
      (`self.Idle`))
    (:`NewEnumerator1`
      (`self.Building` DeltaSeconds))
    (:`NewEnumerator2`
      (`self.Walking`))))

(fn `Building`
  (params (FrameTime :type "Float (double-precision)"))
  (bind _asbuilding (cast `/Game/Blueprints/Building` (`self.AssignedBuilding`)))
  (bind _isbuilt (`/Game/Blueprints/Building.BuildBuilding` _asbuilding (* FrameTime (`self.BuildSpeed`))))
  (if _isbuilt
    (`self.StateSetIdle`)))

(fn `Idle`)

(fn `StateSetBuilding`
  (set `self.State` "NewEnumerator1")
  (`SkeletalMeshComponent.PlayAnimation` (`self.Mesh`) "/Game/Models/Alien/Alien_Anim_AlienRig_Building.Alien_Anim_AlienRig_Building" true))

(fn `StateSetIdle`
  (set `self.State` "NewEnumerator0")
  (`SkeletalMeshComponent.PlayAnimation` (`self.Mesh`) "/Game/Models/Alien/Alien_Anim_AlienRig_Idle.Alien_Anim_AlienRig_Idle" true))

(fn `StateSetWalking`
  (set `self.State` "NewEnumerator2")
  (`SkeletalMeshComponent.PlayAnimation` (`self.Mesh`) "/Game/Models/Alien/Alien_Anim_AlienRig_Idle.Alien_Anim_AlienRig_Idle" true))

(fn `UserConstructionScript`)

(fn `Walking`
  (bind _returnvalue (`self.K2_GetActorLocation`))
  (bind _currentnode (`self.CurrentNode`))
  (bind _position (`GraphNode.Position` (`|GetArrayItem` (`self.Path`) (`self.CurrentNode`))))
  (bind _returnvalue_2 (`KismetMathLibrary.Normal` (- _position _returnvalue)))
  (bind _sweephitresult (`self.K2_SetActorLocationAndRotation` (+ _returnvalue (* (* _returnvalue_2 (`GameplayStatics.GetWorldDeltaSeconds`)) (`self.WalkSpeed`))) (`KismetMathLibrary.MakeRotFromZX` (`KismetMathLibrary.Normal` _returnvalue) _returnvalue_2) true))
  (if (== (`.HitActor` (`GameplayStatics.BreakHitResult` _sweephitresult)) (`self.AssignedBuilding`))
    (`self.StateSetBuilding`)
    (elif (< (`KismetMathLibrary.Vector_Distance` _returnvalue _position) 10.0)
      (if (< _currentnode (- (`KismetArrayLibrary.Array_Length` (`self.Path`)) 1))
        (`/Engine/EditorBlueprintResources/StandardMacros.IncrementInt` _currentnode)
        (else
          (`self.StateSetIdle`))))))

(fn `WalkTo`
  (params (Node :type Integer))
  (bind _nodegraph (`self.NodeGraph`))
  (bind _index (`NodeGraph.GetClosestNode` _nodegraph (`self.K2_GetActorLocation`) 200.0))
  (bind _path (`NodeGraph.Pathfind` _nodegraph _index Node))
  (set `self.Path` _path)
  (set `self.CurrentNode` 1)
  (set `self.State` "NewEnumerator2")
  (`SkeletalMeshComponent.PlayAnimation` (`self.Mesh`) "/Game/Models/Alien/Alien_Anim_AlienRig_Walking.Alien_Anim_AlienRig_Walking" true))