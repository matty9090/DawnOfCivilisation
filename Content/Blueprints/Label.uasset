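; Label is an actor that shows an ObjectTag text widget on screen over its world position.
; It creates the widget on BeginPlay and each tick projects the actor location to screen space to position it.
; A visibility line trace from the camera to the actor hides the tag when the view is blocked.
; A SetVisibility function sets a flag that forces the tag hidden.
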(event `self.ReceiveBeginPlay`
  (bind _returnvalue (`|CreateWidget` "/Game/Blueprints/UI/ObjectTag.ObjectTag_C"))
  (bind _output_get (set `self.TextWidget` _returnvalue))
  (`UserWidget.AddToViewport` _output_get 0))

(event `self.ReceiveTick`
  (params (DeltaSeconds :type "Float (single-precision)"))
  (bind _textwidget (`self.TextWidget`))
  (if (`self.IsHidden`)
    (`Widget.SetVisibility` (`self.TextWidget`) "Hidden")
    (else
      (bind (_outhit _returnvalue) (`KismetSystemLibrary.LineTraceSingle` (`PlayerCameraManager.GetCameraLocation` (`GameplayStatics.GetPlayerCameraManager` 0)) (`self.K2_GetActorLocation`) "TraceTypeQuery1"))
      (if _returnvalue
        (`Widget.SetVisibility` _textwidget "Hidden")
        (else
          (`Widget.SetVisibility` _textwidget "Visible")
          (`UserWidget.SetPositionInViewport` _textwidget (`GameplayStatics.ProjectWorldToScreen` (`GameplayStatics.GetPlayerController` 0) (`self.K2_GetActorLocation`)) true))))))

(fn `SetVisibility`
  (params (Visibility :type Boolean))
  (set `self.IsHidden` (not Visibility)))

(fn `UserConstructionScript`)