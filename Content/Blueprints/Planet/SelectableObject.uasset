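; SelectableObject is a planet Blueprint that gives an object a highlight outline.
; CreateOutlineMesh assigns a supplied static mesh to OutlineMesh and replaces every material slot with the Outline material.
; OnHighlighted and OnUnhighlighted show and hide that mesh without affecting child components.
; The event graph and construction script are empty, so nothing in this Blueprint calls these functions.
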(fn `CreateOutlineMesh`
  (params (Mesh :type "StaticMesh Object Reference"))
  (bind _outlinemesh (`self.OutlineMesh`))
  (`StaticMeshComponent.SetStaticMesh` (`self.OutlineMesh`) Mesh)
  (for (_ _array_index) (`MeshComponent.GetMaterials` _outlinemesh)
    (`PrimitiveComponent.SetMaterial` _outlinemesh _array_index "/Game/Materials/Outline.Outline")))

(fn `OnHighlighted`
  (`SceneComponent.SetVisibility` (`self.OutlineMesh`) true false))

(fn `OnUnhighlighted`
  (`SceneComponent.SetVisibility` (`self.OutlineMesh`) false false))

(fn `UserConstructionScript`)