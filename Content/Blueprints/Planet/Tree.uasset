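; A planet tree that shows an outline when highlighted and belongs to a Forest.
; On BeginPlay it builds an outline mesh from its static mesh.
; Highlight and unhighlight events are forwarded to the Forest rather than applied locally, while separate HighlightTree and UnhighlightTree functions toggle this tree's outline visibility.
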(event `self.ReceiveBeginPlay`
  (`self.CreateOutlineMesh` (`StaticMeshComponent.StaticMesh` (`self.StaticMesh`))))

(event `self.OnHighlighted`
  (`/Game/Blueprints/Planet/Forest.Highlight` (`self.Forest`)))

(event `self.OnUnhighlighted`
  (`/Game/Blueprints/Planet/Forest.Unhighlight` (`self.Forest`)))

(fn `HighlightTree`
  (`SceneComponent.SetVisibility` (`self.OutlineMesh`) true false))

(fn `UnhighlightTree`
  (`SceneComponent.SetVisibility` (`self.OutlineMesh`) false false))

(fn `UserConstructionScript`)