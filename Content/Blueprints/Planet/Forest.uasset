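; Forest actor on the planet that marks a group of trees with a floating screen-space "Forest" name tag.
; CalculatePosition places it at the trees' average location, pushed outward along that direction from the world origin.
; Each tick it projects its location to the viewport to position the ObjectTag widget, hiding it when flagged hidden or when a camera-to-actor visibility trace is blocked.
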(event `self.ReceiveBeginPlay`
  (bind _name (`self.GenerateForestName`))
  (bind _returnvalue (`|CreateWidget` "/Game/Blueprints/UI/ObjectTag.ObjectTag_C" null _name))
  (bind _output_get (set `self.TextWidget` _returnvalue))
  (`UserWidget.AddToViewport` _output_get 0))

(event `self.ReceiveTick`
  (params (DeltaSeconds :type "Float (single-precision)"))
  (bind _textwidget (`self.TextWidget`))
  (if (`self.IsHidden`)
    (`Widget.SetVisibility` (`self.TextWidget`) "Hidden")
    (else
      (bind (_outhit _returnvalue) (`KismetSystemLibrary.LineTraceSingle` (`PlayerCameraManager.GetCameraLocation` (`GameplayStatics.GetPlayerCameraManager` 0)) (`self.K2_GetActorLocation`) "TraceTypeQuery1"))
      (if _returnvalue
        (`Widget.SetVisibility` _textwidget "Hidden")
        (else
          (`Widget.SetVisibility` _textwidget "Visible")
          (`UserWidget.SetPositionInViewport` (`self.TextWidget`) (`GameplayStatics.ProjectWorldToScreen` (`GameplayStatics.GetPlayerController` 0) (`self.K2_GetActorLocation`)) true))))))

(fn `CalculatePosition`
  (locals (TotalLocation :type "Vector Structure"))
  (bind _trees (`self.Trees`))
  (bind _totallocation (`local.TotalLocation`))
  (for _array_element _trees
    (set `local.TotalLocation` (+ (`self.K2_GetActorLocation` _array_element) _totallocation)))
  (`self.K2_SetActorLocation` (+ (/ _totallocation (`KismetArrayLibrary.Array_Length` _trees)) (* (`KismetMathLibrary.Normal` _totallocation) 200.0))))

(fn `GenerateForestName`
  (returns (Name :type String))
  (return "Forest"))

(fn `SetVisibility`
  (params (Visible :type Boolean))
  (set `self.IsHidden` (not Visible)))

(fn `UserConstructionScript`)