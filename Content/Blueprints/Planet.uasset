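; Procedural planet actor built from terrain and water Geosphere child actors, populated with mountains and forests on BeginPlay.
; Mountains displace vertices around random points along their normals using three octaves of ridged simplex noise, then spawn Mountain actors.
; Forests avoid those actors, projecting generated points from a tangent plane by line trace to place trees on near-base-radius terrain.
; Releasing left mouse also spawns a tree where the camera trace hits.
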(event `self.ReceiveBeginPlay`
  (bind _asgeosphere (cast `Geosphere` (`ChildActorComponent.ChildActor` (`self.Terrain`))))
  (set `self.TerrainSphere` _asgeosphere)
  (`self.EnableInput` (`GameplayStatics.GetPlayerController` 0))
  (bind _vertices (`Geosphere.GetVertices` _asgeosphere))
  (`self.AddMountains` _vertices)
  (`self.AddForests` _vertices))

(event `Key|LeftMouseButton`
  (params (Key :type "Key Structure"))
  (bind _returnvalue (`GameplayStatics.GetPlayerCameraManager` 0))
  (bind _returnvalue_2 (`PlayerCameraManager.GetCameraLocation` _returnvalue))
  (:`Released`
    (bind (_outhit _returnvalue_3) (`KismetSystemLibrary.LineTraceSingleForObjects` :`Start` _returnvalue_2 :`End` (+ _returnvalue_2 (* (`self.GetActorForwardVector` _returnvalue) 6000.0)) :`ObjectTypes` (`|MakeArray` "ObjectTypeQuery1" "ObjectTypeQuery2" :!type "EObjectTypeQuery Enum") :`bIgnoreSelf` false))
    (if _returnvalue_3
      (bind (_bblockinghit _binitialoverlap _time _distance _location _impactpoint _normal) (`GameplayStatics.BreakHitResult` _outhit))
      (`|SpawnActorFromClass` "/Game/Blueprints/Tree.Tree_C" (`KismetMathLibrary.MakeTransform` _location (`KismetMathLibrary.MakeRotFromZ` _normal)) "Undefined" "OverrideRootScale" null null))))

(fn `AddForests`
  (params (Vertices :type "Array of Vector Structure"))
  (for _ (range (+ (`self.NumForests`) 1))
    (bind _output_get (set `self.RandomNumber` (`KismetMathLibrary.RandomInteger` (`KismetArrayLibrary.Array_Length` Vertices))))
    (bind _returnvalue (`Geosphere.GetNormal` (`self.TerrainSphere`) _output_get))
    (`self.PlaceForest` (`|GetArrayItem` Vertices _output_get) _returnvalue (`self.ForestRadius`))))

(fn `AddMountain`
  (params (Terrain :type "Geosphere Object Reference") (Vertex :type "Vector Structure") (Normal :type "Vector Structure") (MountainSize :type "Float (double-precision)"))
  (locals (Range :type "Float (double-precision)" :default 500.0))
  (bind (_indices _vertices) (`Geosphere.GetClosestVertices` Terrain Vertex (`local.Range`)))
  (for (_array_element _array_index) _vertices
    (bind _noise (`self.LayeredRidgedNoise` _array_element 0.001))
    (bind _output (`|GetArrayItem` _indices _array_index))
    (bind _returnvalue (`Geosphere.GetNormal` (`local.Terrain`) _output))
    (`Geosphere.SetVertex` (`local.Terrain`) _output (+ _array_element (* _returnvalue (* _noise MountainSize)))))
  (`Geosphere.GenerateMeshSection` Terrain)
  (`|SpawnActorFromClass` "/Game/Blueprints/Mountain.Mountain_C" (`KismetMathLibrary.MakeTransform` (+ Vertex (* Normal 260.0))) "Undefined" "OverrideRootScale" null null))

(fn `AddMountains`
  (params (Vertices :type "Array of Vector Structure"))
  (locals (rndnum :type Integer :default 0))
  (bind _terrainsphere (`self.TerrainSphere`))
  (for _ (range (+ (`self.NumMountains`) 1))
    (bind _output_get (set `local.rndnum` (`KismetMathLibrary.RandomInteger` (`KismetArrayLibrary.Array_Length` Vertices))))
    (bind _returnvalue (`Geosphere.GetNormal` _terrainsphere _output_get))
    (`self.AddMountain` _terrainsphere (`|GetArrayItem` Vertices _output_get) _returnvalue (`self.MountainSize`))))

(fn `IsCloseMountainRange`
  (params (Position :type "Vector Structure") (Threshold :type "Float (double-precision)"))
  (returns (IsMountain :type Boolean))
  (bind _outactors (`GameplayStatics.GetAllActorsOfClass` "/Game/Blueprints/Mountain.Mountain_C"))
  (for _array_element _outactors
    (if (< (`KismetMathLibrary.Vector_Distance` (`self.K2_GetActorLocation` _array_element) (`local.Position`)) (`local.Threshold`))
      (return true)))
  (return false))

(fn `LayeredRidgedNoise`
  (params (pos :type "Vector Structure") (scale :type "Float (double-precision)" :default 0.1))
  (returns (noise :type "Float (double-precision)"))
  (bind _returnvalue (* pos scale))
  (bind _returnvalue_2 (* _returnvalue 2.0))
  (bind _noise (`self.RidgedNoise` _returnvalue))
  (bind _noise_2 (`self.RidgedNoise` _returnvalue_2))
  (bind _noise_3 (`self.RidgedNoise` (* _returnvalue_2 2.0)))
  (return (+ (* _noise 1.0) (* _noise_2 0.5) (* _noise_3 0.25))))

(fn `PlaceForest`
  (params (Position :type "Vector Structure") (Normal :type "Vector Structure") (ForestRadius :type "Float (double-precision)"))
  (locals (Pos :type "Vector Structure") (Points :type "Vector Structure") (StartPoint :type "Vector Structure" :default (0.0 0.0 0.0)) (Axis1 :type "Vector Structure" :default (0.0 0.0 0.0)) (Axis2 :type "Vector Structure" :default (0.0 0.0 0.0)))
  (bind _returnvalue (/ (`self.ForestRadius`) 2.0))
  (bind _ismountain (`self.IsCloseMountainRange` Position ForestRadius))
  (if (not _ismountain)
    (bind _returnvalue_2 (`PoissonDiscSampling.GeneratePoints` (`self.TreeRadius`) ForestRadius (`self.Threshold`) (`self.Frequency`)))
    (set `local.StartPoint` (+ Position (* Normal 300.0)))
    (bind _output_get (set `local.Axis1` (`KismetMathLibrary.Normal` (`KismetMathLibrary.Cross_VectorVector` Normal (0.0 1.0 0.0)))))
    (set `local.Axis2` (`KismetMathLibrary.Normal` (`KismetMathLibrary.Cross_VectorVector` _output_get Normal)))
    (for _array_element _returnvalue_2
      (bind (_x _y) (`KismetMathLibrary.BreakVector2D` _array_element))
      (bind _returnvalue_3 (+ (`local.StartPoint`) (* (`local.Axis1`) (- _x _returnvalue)) (* (`local.Axis2`) (- _y _returnvalue))))
      (bind (_outhit _returnvalue_4) (`KismetSystemLibrary.LineTraceSingle` :`Start` _returnvalue_3 :`End` (+ _returnvalue_3 (* (`local.Normal`) -1000.0)) :`TraceChannel` "TraceTypeQuery1" :`bIgnoreSelf` false :`DrawTime` 60.0))
      (if _returnvalue_4
        (bind (_bblockinghit _binitialoverlap _time _distance _location _impactpoint _normal _impactnormal _physmat _hitactor) (`GameplayStatics.BreakHitResult` _outhit))
        (if (== _hitactor (`ChildActorComponent.ChildActor` (`self.Terrain`)))
          (if (< (- (`KismetMathLibrary.VSize` (- _location (`self.K2_GetActorLocation`))) (`self.Radius`)) 30.0)
            (`|SpawnActorFromClass` "/Game/Blueprints/Tree.Tree_C" (`KismetMathLibrary.MakeTransform` _location (`KismetMathLibrary.MakeRotFromZ` _normal) (0.32 0.32 0.32)) "Undefined" "OverrideRootScale" null null)))))
    (`|SpawnActorFromClass` "/Game/Blueprints/Forest.Forest_C" (`KismetMathLibrary.MakeTransform` (+ (`local.Position`) (* (`local.Normal`) 220.0))) "Undefined" "OverrideRootScale" null null)))

(fn `RidgedNoise`
  (params (pos :type "Vector Structure"))
  (returns (noise :type "Float (double-precision)"))
  (bind _returnvalue (`SimplexNoiseBPLibrary.SimplexNoise3D` (.x pos) (.y pos) (.z pos)))
  (return (* 2.0 (- 0.5 (`KismetMathLibrary.Abs` (- 0.5 _returnvalue))))))

(fn `UserConstructionScript`
  (bind _asgeosphere (cast `Geosphere` (`ChildActorComponent.ChildActor` (`self.Terrain`))))
  (`PrimitiveComponent.SetMaterial` (`Geosphere.Mesh` _asgeosphere) 0 (`self.TerrainMaterial`))
  (bind _asgeosphere_2 (cast `Geosphere` (`ChildActorComponent.ChildActor` (`self.Water`))))
  (`PrimitiveComponent.SetMaterial` (`Geosphere.Mesh` _asgeosphere_2) 0 (`self.WaterMaterial`)))