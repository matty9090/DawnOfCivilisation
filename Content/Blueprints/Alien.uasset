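; Alien character Blueprint that idles on a planet and can request paths across its terrain node graph.
; On BeginPlay it caches the node graph from the Planet's terrain and loops an idle animation on its skeletal mesh.
; WalkTo finds the graph node nearest the alien, within a threshold, and pathfinds to a target node.
; The path result is unused, so no movement happens here.
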(event `self.ReceiveBeginPlay`
  (bind _terrain (`/Game/Blueprints/Planet.GetTerrainRef` (`self.Planet`)))
  (set `self.NodeGraph` (`Geosphere.NodeGraph` _terrain))
  (`SkeletalMeshComponent.PlayAnimation` (`self.SkeletalMeshComponent`) "/Game/Models/Alien/Alien_Anim_AlienRig_Idle.Alien_Anim_AlienRig_Idle" true))

(fn `UserConstructionScript`)

(fn `WalkTo`
  (params (Node :type Integer))
  (bind _nodegraph (`self.NodeGraph`))
  (bind _index (`NodeGraph.GetClosestNode` _nodegraph (`self.K2_GetActorLocation`) 200.0))
  (`NodeGraph.Pathfind` _nodegraph _index Node))