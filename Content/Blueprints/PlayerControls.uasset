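; Player controller for a planet game, handling orbit camera, selection, alien movement and object placement.
; Right-drag rotates the view and the wheel zooms the spring arm within limits.
; Left-click picks an alien, then sends it to the clicked Geosphere node; other selectables get an outline-material duplicate.
; Middle-click spawns SelectedModel oriented outward from world origin, while Z and X mark endpoints and visualize the NodeGraph path with cubes.
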(event `self.ReceiveBeginPlay`)

(event `Key|LeftMouseButton`
  (params (Key :type "Key Structure"))
  (bind (_hitresult _returnvalue) (`self.GetHitResultUnderCursorForObjects` (`|MakeArray` "ObjectTypeQuery1" "ObjectTypeQuery2" "ObjectTypeQuery3" :!type "EObjectTypeQuery Enum")))
  (bind (_bblockinghit _binitialoverlap _time _distance _location _impactpoint _normal _impactnormal _physmat _hitactor) (`GameplayStatics.BreakHitResult` _hitresult))
  (bind _returnvalue_2 (`GameplayStatics.GetObjectClass` _hitactor))
  (bind _returnvalue_3 (`KismetSystemLibrary.GetClassDisplayName` _returnvalue_2))
  (:`Released`
    (if _returnvalue
      (if (== (`self.SelectLocation`) true)
        (set `self.SelectLocation` false)
        (bind _asgeosphere (cast `Geosphere` _hitactor))
        (bind _index (`NodeGraph.GetClosestNode` (`Geosphere.NodeGraph` _asgeosphere) _location 200.0))
        (`/Game/Blueprints/Alien/AlienCharacter.WalkTo` (`self.SelectedAlien`) _index)
        (elif (`self.ActorHasTag` _hitactor "Selectable")
          (`KismetSystemLibrary.PrintString` _returnvalue_3)
          (if (`KismetStringLibrary.EqualEqual_StrStr` _returnvalue_3 "AlienCharacter_C")
            (`KismetSystemLibrary.PrintString` "Select a location")
            (set `self.SelectLocation` true)
            (bind _asalien_character (cast `/Game/Blueprints/Alien/AlienCharacter` _hitactor)
              (:`then`
                (set `self.SelectedAlien` _asalien_character))
              (:`CastFailed`
                (`KismetSystemLibrary.PrintString` "Error casting to alien")))
            (else
              (bind _returnvalue_4 (`|SpawnActorFromClass` _returnvalue_2 (`self.GetTransform` _hitactor) "Undefined" "OverrideRootScale" null null))
              (bind _returnvalue_5 (`self.GetComponentByClass` _returnvalue_4 "/Script/Engine.StaticMeshComponent"))
              (if (`KismetSystemLibrary.IsValid` _returnvalue_5)
                (for (_ _array_index) (`MeshComponent.GetMaterials` _returnvalue_5)
                  (`PrimitiveComponent.SetMaterial` _returnvalue_5 _array_index "/Game/Materials/Outline.Outline"))))))))))

(event `Key|Z`
  (params (Key :type "Key Structure"))
  (bind (_hitresult _returnvalue) (`self.GetHitResultUnderCursorForObjects` (`|MakeArray` "ObjectTypeQuery1" "ObjectTypeQuery2" "ObjectTypeQuery3" :!type "EObjectTypeQuery Enum")))
  (bind (_bblockinghit _binitialoverlap _time _distance _location _impactpoint _normal _impactnormal _physmat _hitactor) (`GameplayStatics.BreakHitResult` _hitresult))
  (:`Released`
    (if _returnvalue
      (bind _asgeosphere (cast `Geosphere` _hitactor))
      (bind (_index _vertex) (`NodeGraph.GetClosestNode` (`Geosphere.NodeGraph` _asgeosphere) _location 200.0))
      (set `self.StartNode` _index)
      (`|SpawnActorFromClass` "/Game/Blueprints/Cube_Blueprint.Cube_Blueprint_C" (`KismetMathLibrary.MakeTransform` _vertex (struct) (0.2 0.2 0.2)) "Undefined" "OverrideRootScale" null null))))

(event `Key|X`
  (params (Key :type "Key Structure"))
  (bind (_hitresult _returnvalue) (`self.GetHitResultUnderCursorForObjects` (`|MakeArray` "ObjectTypeQuery1" "ObjectTypeQuery2" "ObjectTypeQuery3" :!type "EObjectTypeQuery Enum")))
  (bind (_bblockinghit _binitialoverlap _time _distance _location _impactpoint _normal _impactnormal _physmat _hitactor) (`GameplayStatics.BreakHitResult` _hitresult))
  (:`Released`
    (if _returnvalue
      (bind _asgeosphere (cast `Geosphere` _hitactor))
      (bind (_index _vertex) (`NodeGraph.GetClosestNode` (`Geosphere.NodeGraph` _asgeosphere) _location 200.0))
      (set `self.EndNode` _index)
      (`|SpawnActorFromClass` "/Game/Blueprints/Cube_Blueprint.Cube_Blueprint_C" (`KismetMathLibrary.MakeTransform` _vertex (struct) (0.2 0.2 0.2)) "Undefined" "OverrideRootScale" null null)
      (bind (_path _returnvalue_2) (`NodeGraph.Pathfind` (`Geosphere.NodeGraph` _asgeosphere) (`self.StartNode`) (`self.EndNode`)))
      (if _returnvalue_2
        (for _array_element _path
          (`|SpawnActorFromClass` "/Game/Blueprints/Cube_Blueprint.Cube_Blueprint_C" (`KismetMathLibrary.MakeTransform` (`GraphNode.Position` _array_element) (struct) (0.2 0.2 0.2)) "Undefined" "OverrideRootScale" null null))))))

(event `Key|MiddleMouseButton`
  (params (Key :type "Key Structure"))
  (bind (_hitresult _returnvalue) (`self.GetHitResultUnderCursorByChannel` "TraceTypeQuery3" false))
  (bind (_bblockinghit _binitialoverlap _time _distance _location _impactpoint _normal _impactnormal _physmat _hitactor _hitcomponent _hitbonename _hititem _faceindex _tracestart _traceend) (`GameplayStatics.BreakHitResult` _hitresult))
  (:`Released`
    (if _returnvalue
      (`KismetSystemLibrary.LineTraceSingle` :`Start` _tracestart :`End` _traceend :`TraceChannel` "TraceTypeQuery3" :`DrawTime` 20.0)
      (`|SpawnActorFromClass` (`self.SelectedModel`) (`KismetMathLibrary.MakeTransform` _location (`KismetMathLibrary.MakeRotFromZ` (`KismetMathLibrary.Normal` _location))) "AlwaysSpawn" "OverrideRootScale" _hitactor null))))

(event `InputAxisKey|MouseWheelAxis`
  (params (AxisValue :type "Float (single-precision)"))
  (bind _returnvalue (`self.GetComponentByClass` (`GameplayStatics.GetPlayerCharacter` 0) "/Script/Engine.SpringArmComponent"))
  (bind _returnvalue_2 (+ (`SpringArmComponent.TargetArmLength` _returnvalue) (* AxisValue -180.0)))
  ;[1 1 1] Scroll wheel to zoom in/out of planet
  (if (`KismetMathLibrary.InRange_FloatFloat` _returnvalue_2 4000.0 8000.0)
    (set `SpringArmComponent.TargetArmLength` _returnvalue_2 _returnvalue)))

(event `InputAxisKey|MouseX`
  (params (AxisValue :type "Float (single-precision)"))
  (bind (_deltax _deltay) (`self.GetInputMouseDelta`))
  ;[1 1 1] Arcball rotation around planet
  (if (`self.MousePress`) :!label _label
    (`self.AddYawInput` _deltax)
    (`self.AddPitchInput` (* -1 _deltay))))

(event `InputAxisKey|MouseY`
  (params (AxisValue :type "Float (single-precision)"))
  ;[1 1 1] Arcball rotation around planet
  (goto _label))

(event `Key|RightMouseButton`
  (params (Key :type "Key Structure"))
  ;[1 1 1] Only rotate around planet when holding left mouse button
  (:`Pressed`
    (set `self.MousePress` true)
    (set `self.bShowMouseCursor` false))
  (:`Released`
    (set `self.MousePress` false)
    (set `self.bShowMouseCursor` true)))

(fn `UserConstructionScript`)