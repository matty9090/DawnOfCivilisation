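; Game Blueprint that passes completed milestones to the UI for display.
; OnMilestoneCompleted switches on the milestone type to format its data, adding an "unlocked!" suffix for buildings and technologies and showing achievement data as is.
; The milestone name and formatted text go to UI.DisplayMilestone as title and description.
; The Tick function is empty.
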(event `self.OnMilestoneCompleted`
  (params (milestoneEvt :type "GameEvent Structure"))
  (bind (_name _energyconsumption _type _data) (break `GameEvent` milestoneEvt))
  (bind _returnvalue (`KismetTextLibrary.Conv_StringToText` _data))
  (switch `EEvent` _type
    (:`UnlockBuilding`
      (set `self.MilestoneText` (`KismetTextLibrary.Conv_TextToString` (`|FormatText` "{0} unlocked!" _returnvalue))))
    (:`UnlockTechnology`
      (set `self.MilestoneText` (`KismetTextLibrary.Conv_TextToString` (`|FormatText` "{0} unlocked!" _returnvalue))))
    (:`Achievement`
      (set `self.MilestoneText` (`KismetTextLibrary.Conv_TextToString` (`|FormatText` "{0}" _returnvalue)))))
  (`/Game/Blueprints/UI/UI.DisplayMilestone` (`self.UI`) _name (`self.MilestoneText`)))

(fn `Tick`)