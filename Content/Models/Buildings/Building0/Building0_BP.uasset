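; Building0_BP is a constructible building that changes its mesh once enough build progress has been added.
; BuildBuilding adds an amount to BuildingProgress and returns whether it has reached MaxProgress.
; Tick polls for progress strictly exceeding MaxProgress, then calls SetBuilt through a DoOnce.
; SetBuilt applies BuildingMesh and completes the "Mr Miner" milestone on the GameManager reached through PlayerControls.
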(event `self.ReceiveTick`
  (params (DeltaSeconds :type "Float (single-precision)"))
  (if (> (`self.BuildingProgress`) (`self.MaxProgress`))
    (`/Engine/EditorBlueprintResources/StandardMacros.DoOnce` false
      (:`Completed`
        (`self.SetBuilt`)))))

(fn `BuildBuilding`
  (params (BuildAmount :type "Float (double-precision)"))
  (returns (IsBuilt :type Boolean))
  (bind _output_get (set `self.BuildingProgress` (+ BuildAmount (`self.BuildingProgress`))))
  (return (>= _output_get (`self.MaxProgress`))))

(fn `SetBuilt`
  (`StaticMeshComponent.SetStaticMesh` (`self.StaticMesh`) (`self.BuildingMesh`))
  (bind _asplayer_controls (cast `/Game/Blueprints/PlayerControls` (`GameplayStatics.GetPlayerController` 0)))
  (`GameManager.CompleteMilestone` (`/Game/Blueprints/PlayerControls.GameManager` _asplayer_controls) "Mr Miner"))

(fn `UserConstructionScript`)